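; BP_MainMenuMode is the FogScape main menu mode Blueprint that shows and removes the main menu widget.
; On BeginPlay it creates WBP_MainMenu, adds it to the player screen, sets UI-only input focused on the widget, and shows the mouse cursor.
; CloseMenu, meant to run before a level loads, restores game-only input, hides the cursor, removes the widget and clears its reference.
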(event Custom|CloseMenu
  (bind _returnvalue (Game|GetPlayerController 0))
  ;[1 0.3 0.2702] Closing main menu before loading level
  (Input|SetInputModeGameOnly _returnvalue false)
  (Variables|/Script/Engine.PlayerController|SetbShowMouseCursor _returnvalue false)
  (Widget|RemovefromParent (Variables|Default|GetMainMenuWidget))
  (Variables|Default|SetMainMenuWidget 0))

(event EventBeginPlay
  (bind _returnvalue (Game|GetPlayerController 0))
  ;[0.4247 1 0.3851] Opening main menu on startup
  (bind _returnvalue_2 (UserInterface|CreateWidget "/Game/FogScape/UI/WBP_MainMenu.WBP_MainMenu_C"))
  (bind _output_get (Variables|Default|SetMainMenuWidget _returnvalue_2))
  (UserInterface|Viewport|AddtoPlayerScreen _output_get)
  (Input|SetInputModeUIOnly _returnvalue (Variables|Default|GetMainMenuWidget) "DoNotLock" false)
  (Variables|/Script/Engine.PlayerController|SetbShowMouseCursor _returnvalue true))

(event EventTick
  (params (DeltaSeconds :type Float%20%28single-precision%29)))

(fn ConstructionScript)