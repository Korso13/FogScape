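; Player controller that drives BP_MainCharacter through Enhanced Input, adding its mapping context shortly after BeginPlay.
; Look input yaws the character mesh and pitches the camera, and movement follows the mesh's yaw.
; Interact toggles glove use to grab and release objects, with another action sliding the grab point to push or pull them.
; Open and close functions manage the Building01 briefing widget, switching input mode and cursor; look is blocked while it exists.
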(event Input|EnhancedActionEvents|EnhancedInputActionIA_MoveFrwdBackward
  (params (ActionValue :type Float%20%28double-precision%29) (ElapsedSeconds :type Float%20%28double-precision%29) (TriggeredSeconds :type Float%20%28double-precision%29) (InputAction :type Input%20Action%20Object%20Reference :default "/Game/FogScape/Blueprints/Core/Controls/IA_MoveFrwdBackward.IA_MoveFrwdBackward"))
  ;[1 1 1] Player Movement mapping
  (:Triggered
    (Pawn|Input|AddMovementInput (Variables|Default|GetPlayerPawn) (Math|Vector|GetForwardVector (Math|Rotator|MakeRotator 0.0 0.0 (.yaw (Transformation|GetWorldRotation (Variables|/Script/Engine.Character|GetMesh (Variables|Default|GetPlayerPawn)))))) ActionValue false)))

(event Input|EnhancedActionEvents|EnhancedInputActionIA_Strafe
  (params (ActionValue :type Float%20%28double-precision%29) (ElapsedSeconds :type Float%20%28double-precision%29) (TriggeredSeconds :type Float%20%28double-precision%29) (InputAction :type Input%20Action%20Object%20Reference :default "/Game/FogScape/Blueprints/Core/Controls/IA_Strafe.IA_Strafe"))
  ;[1 1 1] Player Movement mapping
  (:Triggered
    (Pawn|Input|AddMovementInput (Variables|Default|GetPlayerPawn) (Math|Vector|GetRightVector (Math|Rotator|MakeRotator 0.0 0.0 (.yaw (Transformation|GetWorldRotation (Variables|/Script/Engine.Character|GetMesh (Variables|Default|GetPlayerPawn)))))) ActionValue false)))

(event Input|EnhancedActionEvents|EnhancedInputActionIA_PullPushObject_Glove
  (params (ActionValue :type Float%20%28double-precision%29) (ElapsedSeconds :type Float%20%28double-precision%29) (TriggeredSeconds :type Float%20%28double-precision%29) (InputAction :type Input%20Action%20Object%20Reference :default "/Game/FogScape/Blueprints/Core/Controls/IA_PullPushObject_Glove.IA_PullPushObject_Glove"))
  (bind _playerpawn (Variables|Default|GetPlayerPawn))
  (bind _grabpoint (Variables|/Game/FogScape/Blueprints/Core/BP_MainCharacter.BP_MainCharacter_C|GetGrabPoint _playerpawn))
  ;[0.3086 0.1435 1] Pull\Push grabbed object
  (:Triggered
    (Variables|/Game/FogScape/Blueprints/Core/BP_MainCharacter.BP_MainCharacter_C|GetGrabbed%20Actor _playerpawn
      (:then
        (Transformation|AddWorldOffset _grabpoint (* (Math|Vector|GetForwardVector _grabpoint) ActionValue) false false))
      (:else))))

(event Input|EnhancedActionEvents|EnhancedInputActionIA_Interact
  (params (ActionValue :type Boolean) (ElapsedSeconds :type Float%20%28double-precision%29) (TriggeredSeconds :type Float%20%28double-precision%29) (InputAction :type Input%20Action%20Object%20Reference :default "/Game/FogScape/Blueprints/Core/Controls/IA_Interact.IA_Interact"))
  (bind _playerpawn (Variables|Default|GetPlayerPawn))
  ;[1 1 1] Player interaction mapping
  (:Triggered
    (Utilities|FlowControl|Sequence
      (:then_0
        (Variables|/Game/FogScape/Blueprints/Core/BP_MainCharacter.BP_MainCharacter_C|SetbUsesGlove _playerpawn true :!label _label))
      (:then_1
        (Default|GrabObject _playerpawn))))
  (:Started
    (Development|PrintString "Interacting")
    (goto _label))
  (:Completed
    (Variables|/Game/FogScape/Blueprints/Core/BP_MainCharacter.BP_MainCharacter_C|SetbUsesGlove (Variables|Default|GetPlayerPawn) false)
    (Default|TryRelease _playerpawn)))

(event Input|EnhancedActionEvents|EnhancedInputActionIA_Jump
  (params (ActionValue :type Boolean) (ElapsedSeconds :type Float%20%28double-precision%29) (TriggeredSeconds :type Float%20%28double-precision%29) (InputAction :type Input%20Action%20Object%20Reference :default "/Game/FogScape/Blueprints/Core/Controls/IA_Jump.IA_Jump"))
  ;[1 1 1] Player jump controlls
  (:Started
    (Character|Jump (Variables|Default|GetPlayerPawn))))

(event Input|EnhancedActionEvents|EnhancedInputActionIA_Look
  (params (ActionValue :type Vector%202D%20Structure) (ElapsedSeconds :type Float%20%28double-precision%29) (TriggeredSeconds :type Float%20%28double-precision%29) (InputAction :type Input%20Action%20Object%20Reference :default "/Game/FogScape/Blueprints/Core/Controls/IA_Look.IA_Look"))
  (bind _playerpawn (Variables|Default|GetPlayerPawn))
  ;[1 1 1] Player camera controls
  (:Triggered
    (Variables|Default|GetBriefing%20Window
      (:then)
      (:else
        (Transformation|AddRelativeRotation (Variables|/Script/Engine.Character|GetMesh _playerpawn) (Math|Rotator|MakeRotator 0.0 0.0 (.x ActionValue)) false false)
        (Transformation|AddRelativeRotation (Variables|/Game/FogScape/Blueprints/Core/BP_MainCharacter.BP_MainCharacter_C|GetCamera _playerpawn) (Math|Rotator|MakeRotator 0.0 (.y ActionValue) 0.0) false false)))))

(event EventBeginPlay
  ;[1 1 1] Enable controlls mapping
  (Utilities|FlowControl|Delay 0.2)
  (bind _asbp_main_character (Utilities|Casting|CastToBP_MainCharacter (Game|GetPlayerCharacter 0)))
  (Variables|Default|SetPlayerPawn _asbp_main_character)
  (Input|AddMappingContext (PlayerController|LocalPlayerSubsystems|GetEnhancedInputLocalPlayerSubsystem self) "/Game/FogScape/Blueprints/Core/Controls/IMC_MainCharControl.IMC_MainCharControl" 0 "(bIgnoreAllPressedKeysUntilRelease=True,bForceImmediately=False)"))

(event EventTick
  (params (DeltaSeconds :type Float%20%28single-precision%29)))

(fn ConstructionScript)

(fn OpenBriefingWidget
  (Variables|Default|GetBriefing%20Window
    (:then)
    (:else
      (bind _returnvalue (UserInterface|CreateWidget "/Game/FogScape/UI/WBP_Building01_Briefing.WBP_Building01_Briefing_C"))
      (bind _output_get (Variables|Default|SetBriefing%20Window _returnvalue))
      (UserInterface|Viewport|AddtoPlayerScreen _output_get)
      (Input|SetInputModeUIOnly self (Variables|Default|GetBriefing%20Window) "DoNotLock" true)
      (Variables|Default|SetbShowMouseCursor true))))

(fn CloseBriefingWidget
  (bind _briefing_window (Variables|Default|GetBriefing%20Window)
    (:then
      (Widget|RemovefromParent _briefing_window)
      (Input|SetInputModeGameOnly self true)
      (Variables|Default|SetbShowMouseCursor false)
      (Variables|Default|SetBriefing%20Window 0))
    (:else)))