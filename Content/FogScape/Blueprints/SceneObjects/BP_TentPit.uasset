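; BP_TentPit is a tentacle pit scene object that grows tentacles linked to nearby physics bodies.
; On BeginPlay it sphere-traces around its Base for physics-body actors that carry a BPC_AttachPoint component, with debug drawing on.
; For each valid hit it spawns a Tentacle skeletal mesh at Base, then attaches that actor's attach-point component to the tentacle's end socket.
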(event EventBeginPlay
  (bind _base (Variables|Default|GetBase))
  (bind _returnvalue (Transformation|GetWorldLocation _base))
  (bind (_outhits _returnvalue_2) (Collision|MultiSphereTraceForObjects _returnvalue (+ _returnvalue "0.000000,0.000000,1.000000") 3e+02 (Utilities|Array|MakeArray "ObjectTypeQuery4") false 0 "ForDuration"))
  (if _returnvalue_2
    (for _array_element _outhits
      (bind _output_get (Variables|Default|SetFound%20Attach%20Point (Actor|GetComponentbyClass (.hitactor _array_element) "/Game/FogScape/Blueprints/Components/BPC_AttachPoint.BPC_AttachPoint_C")))
      (if (Utilities|IsValid _output_get)
        (bind _returnvalue_3 (AddComponent|AddSkeletalMeshComponent false))
        (Utilities|Array|Add (Variables|Default|GetTentacles) _returnvalue_3)
        (Components|SkeletalMesh|SetSkeletalMeshAsset _returnvalue_3 "/Game/FogScape/Meshes/Tent/Tentacle.Tentacle")
        (Transformation|AttachComponentToComponent _returnvalue_3 (Variables|Default|GetBase) "None" "SnapToTarget" "SnapToTarget" "KeepRelative" true)
        (Transformation|AttachComponentToComponent (Actor|GetComponentbyClass (.hitactor _array_element) "/Game/FogScape/Blueprints/Components/BPC_AttachPoint.BPC_AttachPoint_C") _returnvalue_3 "DEF_Tentacle_013_endSocket" "KeepRelative" "KeepRelative" "KeepRelative" true)))))

(event Collision|EventActorBeginOverlap
  (params (OtherActor :type Actor%20Object%20Reference)))

(event EventTick
  (params (DeltaSeconds :type Float%20%28single-precision%29)))

(fn ConstructionScript)